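; DialogGoddesPlanFixBP is an Actor Blueprint that steps through an array of dialog lines for a text block.
; StartStoryTeller only stores the incoming lines.
; RunStoryTeller advances the index, waits between lines after the first, clears the text block, resets the finish-now flag and stores the current line as a string.
; The graph shows neither a call to RunStoryTeller nor the code that displays that string.
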(event Custom|StartStoryTeller
  (params (TextToDisplay :type Array%20of%20Texts))
  ;[1 1 1] Call for initial method
  (Variables|Default|SetTextToDisplay TextToDisplay))

(event Custom|RunStoryTeller
  (bind _result (Math|Integer|IncrementInt (Variables|Default|GetarrayIterator))
    (:%20%20
      (Variables|Default|SetarrayIterator _result)
      (if (not (>= (Variables|Default|GetarrayIterator) (Utilities|Array|Length (Variables|Default|GetTextToDisplay))))
        (if (> (Variables|Default|GetarrayIterator) 0)
          (Utilities|FlowControl|Delay (Variables|Default|GetdelayBetweenLines)))
        (Rendering|Components|TextRender|SetText (Variables|Default|GetTextBlock) "")
        (Variables|Default|SetfinishTextNow false)
        (Variables|Default|SetcurrentStringToDisplay (Utilities|String|ToString(Text) (Utilities|Array|Get(acopy) (Variables|Default|GetTextToDisplay) (Variables|Default|GetarrayIterator))))))))

(event EventBeginPlay)

(event Collision|EventActorBeginOverlap
  (params (OtherActor :type Actor%20Object%20Reference)))

(event EventTick
  (params (DeltaSeconds :type Float%20%28single-precision%29)))

(fn ConstructionScript)